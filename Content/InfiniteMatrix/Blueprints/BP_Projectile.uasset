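; Player projectile that flies along world X, destroys enemies on overlap and awards streak-based score.
; FireProjectile sets its speed to three times the supplied player speed, and Tick applies the movement as a world offset.
; Enemy hits raise the player's streak, which feeds the score and cooldown widget display.
; Other non-player overlaps reset the streak and destroy the projectile, while a short lifetime timeout destroys it without resetting.
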(event `self.ReceiveBeginPlay`
  (`KismetSystemLibrary.Delay` 3.0)
  (`self.K2_DestroyActor`))

(event `self.ReceiveActorBeginOverlap`
  (params (OtherActor :type "Actor Object Reference"))
  (bind _player (`self.Player`))
  (cast `/Game/InfiniteMatrix/Blueprints/BP_Player` OtherActor
    (:`CastFailed`
      (bind _asbp_enemy (cast `/Game/InfiniteMatrix/Blueprints/BP_Enemy` OtherActor)
        (:`then`
          (`self.K2_DestroyActor` _asbp_enemy)
          (bind _result (`/Engine/EditorBlueprintResources/StandardMacros.IncrementInt` (`/Game/InfiniteMatrix/Blueprints/BP_Player.ProjectileStreak` _player))
            (:`  `
              (`/Game/InfiniteMatrix/Blueprints/BP_Player.IncreaseScore` _player _result)
              (`/Game/InfiniteMatrix/UI/WBP_ProjectileCooldown.DisplayProjectileScore` (`/Game/InfiniteMatrix/Blueprints/BP_Player.CooldownWidget` _player) _result))))
        (:`CastFailed`
          (set `/Game/InfiniteMatrix/Blueprints/BP_Player.ProjectileStreak` 0 _player)))
      (`self.K2_DestroyActor`))))

(event `self.ReceiveTick`
  (params (DeltaSeconds :type "Float (single-precision)"))
  (`self.K2_AddActorWorldOffset` (`KismetMathLibrary.MakeVector` (* DeltaSeconds (`self.Speed`)))))

(fn `FireProjectile`
  (params (PlayerSpeed :type "Float (double-precision)"))
  (set `self.Speed` (* PlayerSpeed 3.0)))

(fn `UserConstructionScript`)