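; BP_HealthPackSpawner is a helper Blueprint that randomly places health pack pickups relative to a given tunnel location.
; AttemptSpawnHealthPack takes a tunnel location and, on a one-in-four roll, spawns a BP_HealthPack at a random distance forward along world X with random Y and Z jitter.
; The event graph and construction script are empty, so spawning happens only when that function is called.
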(fn `AttemptSpawnHealthPack`
  (params (TunnelLocation :type "Vector Structure"))
  (locals (NewLocalVar :type "Vector Structure"))
  (if (< (`KismetMathLibrary.RandomFloat`) 0.25)
    (bind _output_get (set `local.NewLocalVar` TunnelLocation))
    (`|SpawnActorFromClass` "/Game/InfiniteMatrix/Blueprints/BP_HealthPack.BP_HealthPack_C" (`KismetMathLibrary.MakeTransform` (`KismetMathLibrary.MakeVector` (+ (.x _output_get) (`KismetMathLibrary.RandomFloatInRange` 700.0 1800.0)) (+ (.y _output_get) (`KismetMathLibrary.RandomFloatInRange` -200.0 200.0)) (+ (.z _output_get) (`KismetMathLibrary.RandomFloatInRange` -200.0 200.0)))) "Undefined" "MultiplyWithRoot" null null)))

(fn `UserConstructionScript`)